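; Terrain tile for an infinite, chained level that scatters props and foliage on itself at BeginPlay through PlaceActors.
; Player entry into LockingVolume closes the back barrier and asks InfiniteTerrainGameMode to spawn the next indexed tile.
; Leaving LockingVolume hides the front barrier while the back stays solid, and entering DestroyingVolume destroys the tile.
; An Arrow exposes the attach transform, and the tile index affects initial red-barrier visibility.
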(event `self.ReceiveBeginPlay`
  (`self.Start Unlock`)
  (`self.PlaceActors` "/Game/Dynamic/Terrain/Props/BP_Container.BP_Container_C" 1 1 400.0)
  (`self.PlaceActors` "/Game/Dynamic/Terrain/Props/BP_Barrel.BP_Barrel_C" 4 7 30.0)
  (`self.PlaceActors` "/Game/Dynamic/Terrain/Props/BP_CherryTree.BP_CherryTree_C" 4 5 50.0)
  (`self.PlaceActors` "/Game/Dynamic/Terrain/Props/BP_PlainsGrass01.BP_PlainsGrass01_C" 50 60 1.0)
  (`self.PlaceActors` "/Game/Dynamic/Terrain/Props/BP_PlainsFern03.BP_PlainsFern03_C" 5 7 10.0)
  (`self.PlaceActors` "/Game/Dynamic/Terrain/Props/BP_Sacks.BP_Sacks_C" 1 2 100.0)
  (`self.PlaceActors` "/Game/Dynamic/Terrain/Props/BP_PlainsFern02.BP_PlainsFern02_C" 4 7 10.0)
  (`self.PlaceActors` "/Game/Dynamic/Terrain/Props/BP_ExoCartIntact.BP_ExoCartIntact_C" 1 2 180.0)
  (`self.PlaceActors` "/Game/Dynamic/Terrain/Props/BP_PlainsSmallRock2.BP_PlainsSmallRock2_C" 4 7 400.0 1.0 5.0)
  (`self.PlaceActors` "/Game/Dynamic/Terrain/Props/BP_Grass01.BP_Grass01_C" 20 30 0.5)
  (`self.PlaceActors` "/Game/Dynamic/Terrain/Props/BP_Grass02.BP_Grass02_C" 20 30 0.5)
  (`self.PlaceActors` "/Game/Dynamic/Terrain/Props/BP_Grass05.BP_Grass05_C" 20 30 0.5 1.0 5.0))

(event `self.Locking Volume.OnComponentBeginOverlap`
  (params (OverlappedComponent :type "PrimitiveComponent Object Reference") (OtherActor :type "Actor Object Reference") (OtherComp :type "PrimitiveComponent Object Reference") (OtherBodyIndex :type Integer) (bFromSweep :type Boolean) (SweepResult :type "HitResult Structure (by ref)"))
  (`self.Is player Actor` OtherActor)
  (`self.Unlock`)
  (`self.Spawn a Tile`))

(event `self.Locking Volume.OnComponentEndOverlap`
  (params (OverlappedComponent :type "PrimitiveComponent Object Reference") (OtherActor :type "Actor Object Reference") (OtherComp :type "PrimitiveComponent Object Reference") (OtherBodyIndex :type Integer))
  (`self.Is player Actor` OtherActor)
  (`self.Lock`))

(event `self.Destroying Volume.OnComponentBeginOverlap`
  (params (OverlappedComponent :type "PrimitiveComponent Object Reference") (OtherActor :type "Actor Object Reference") (OtherComp :type "PrimitiveComponent Object Reference") (OtherBodyIndex :type Integer) (bFromSweep :type Boolean) (SweepResult :type "HitResult Structure (by ref)"))
  (`self.Is player Actor` OtherActor)
  (`self.K2_DestroyActor`))

(fn `Get Attach Location`
  (returns (`Attach Transform` :type "Transform Structure"))
  (return (`SceneComponent.K2_GetComponentToWorld` (`self.Arrow`))))

(fn `Get Index of Tile`
  (returns (Index :type Integer))
  (return (`self.IndexOfTile`)))

(fn `Lock`
  (bind _back_barrier (`self.Back_Barrier`))
  (bind _frontbarrier (`self.FrontBarrier`))
  (`PrimitiveComponent.SetCollisionEnabled` _back_barrier "QueryAndPhysics")
  (`SceneComponent.SetVisibility` _back_barrier true false)
  (`PrimitiveComponent.SetCollisionEnabled` _frontbarrier "NoCollision")
  (`SceneComponent.SetVisibility` _frontbarrier false false))

(fn `Set Index of Tile`
  (params (Index :type Integer))
  (`self.Set Index of Tile` Index)
  (return))

(fn `Spawn a Tile`
  (bind _asinfinite_terrain_game_mode (cast `/Game/Dynamic/GameMode/InfiniteTerrainGameMode` (`GameplayStatics.GetGameMode`)))
  (bind _tile_index (`/Game/Dynamic/GameMode/InfiniteTerrainGameMode.Get Tile Index` _asinfinite_terrain_game_mode))
  (bind _returnvalue (+ _tile_index 1))
  (`KismetSystemLibrary.PrintString` (`KismetStringLibrary.Concat_StrStr` "Spawn " (`KismetStringLibrary.Conv_IntToString` _returnvalue) " Tile!"))
  (`/Game/Dynamic/GameMode/InfiniteTerrainGameMode.Spawn Tile` _asinfinite_terrain_game_mode _returnvalue)
  (return))

(fn `Start Unlock`
  (bind _frontbarrier (`self.FrontBarrier`))
  (bind _frontredbarrier (`self.FrontRedBarrier`))
  (bind _back_barrier (`self.Back_Barrier`))
  (`PrimitiveComponent.SetCollisionEnabled` _back_barrier "NoCollision")
  (`SceneComponent.SetVisibility` _back_barrier false false)
  (`PrimitiveComponent.SetCollisionEnabled` _frontbarrier "NoCollision")
  (`SceneComponent.SetVisibility` _frontbarrier true false)
  (`PrimitiveComponent.SetCollisionEnabled` _frontredbarrier "NoCollision")
  (if (<= (`self.IndexOfTile`) 1)
    (`SceneComponent.SetVisibility` _frontredbarrier false false)))

(fn `Unlock`
  (bind _frontredbarrier (`self.FrontRedBarrier`))
  (bind _back_barrier (`self.Back_Barrier`))
  (bind _frontbarrier (`self.FrontBarrier`))
  (`PrimitiveComponent.SetCollisionEnabled` _back_barrier "QueryAndPhysics")
  (`SceneComponent.SetVisibility` _back_barrier true false)
  (`PrimitiveComponent.SetCollisionEnabled` _frontbarrier "NoCollision")
  (`SceneComponent.SetVisibility` _frontbarrier true false)
  (`PrimitiveComponent.SetCollisionEnabled` _frontredbarrier "NoCollision")
  (`SceneComponent.SetVisibility` _frontredbarrier false false))

(fn `UserConstructionScript`)