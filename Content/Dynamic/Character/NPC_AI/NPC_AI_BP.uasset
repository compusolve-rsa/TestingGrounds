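; AI controller for guard NPCs that starts patrol behavior and tracks perceived non-guard actors as enemies.
; On BeginPlay it sets up the PatrolData blackboard and runs the GuardBehaviour behavior tree.
; AI perception updates write sensed actors without the Guard tag to the blackboard's enemy key.
; A lost-sense update for such an actor clears that key.
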(event `self.ReceiveBeginPlay`
  ;[1 1 1] Begin Patrolling Behavior
  (bind _blackboardcomponent (`self.UseBlackboard` "/Game/Dynamic/Character/NPC_AI/PatrolData.PatrolData"))
  (`self.RunBehaviorTree` "/Game/Dynamic/Character/NPC_AI/GuardBehaviour.GuardBehaviour")
  (set `self.BlackBoardComp` _blackboardcomponent))

(event `self.AIPerception.OnTargetPerceptionUpdated`
  (params (Actor :type "Actor Object Reference") (Stimulus :type "AIStimulus Structure"))
  (`self.Update BlackBord Enemy Key` Actor Stimulus Actor))

(fn `Update BlackBord Enemy Key`
  (params (ObjectValue :type "Object Object Reference") (AIStimulus :type "AIStimulus Structure (by ref)") (self2 :type "Actor Object Reference"))
  (bind _blackboardcomp (`self.BlackBoardComp`))
  (bind _enemykey (`self.EnemyKey`))
  (if (`self.ActorHasTag` self2 "Guard")
    _
    (elif (`.bSuccessfullySensed` (break `AIStimulus` AIStimulus))
      (`BlackboardComponent.SetValueAsObject` _blackboardcomp _enemykey ObjectValue)
      (else
        (`BlackboardComponent.ClearValue` _blackboardcomp _enemykey)))))

(fn `UserConstructionScript`)