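; AI controller Blueprint for guard NPCs that perceive and track non-guard actors.
; On BeginPlay it sets up the PatrolData blackboard, runs the GuardBehaviour behavior tree and caches the blackboard component.
; AI Perception updates ignore actors tagged Guard, writing any other sensed actor to the enemy key and clearing that key when sensing fails.
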(event `self.ReceiveBeginPlay`
  (bind _blackboardcomponent (`self.UseBlackboard` "/Game/NPC/NPC_AI/PatrolData.PatrolData"))
  (`self.RunBehaviorTree` "/Game/NPC/NPC_AI/GuardBehaviour.GuardBehaviour")
  (set `self.BlackBoardComp` _blackboardcomponent))

(event `self.AIPerception.OnTargetPerceptionUpdated`
  (params (Actor :type "Actor Object Reference") (Stimulus :type "AIStimulus Structure"))
  (bind _blackboardcomp (`self.BlackBoardComp`))
  (bind _enemykey (`self.EnemyKey`))
  (if (`self.ActorHasTag` Actor "Guard")
    _
    (elif (`.bSuccessfullySensed` (break `AIStimulus` Stimulus))
      (`BlackboardComponent.SetValueAsObject` _blackboardcomp _enemykey Actor)
      (else
        (`BlackboardComponent.ClearValue` _blackboardcomp _enemykey)))))

(fn `UserConstructionScript`)